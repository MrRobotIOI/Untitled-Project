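; BP_MeteorSpawnArea is a box area actor meant to periodically spawn BP_Meteor actors.
; Tick calls SpawnMeteor whenever the named spawn cooldown is off, then updates the cooldown array by delta time.
; SpawnMeteor's entry is unwired, so it currently does nothing.
; Its disconnected nodes would restart the cooldown and spawn a meteor at a random point in the actor-scaled box with randomised pitch.
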(event EventBeginPlay)

(event Collision|EventActorBeginOverlap
  (params (OtherActor :type Actor%20Object%20Reference)))

(event EventTick
  (params (DeltaSeconds :type Float%20%28single-precision%29))
  (Utilities|FlowControl|Sequence
    (:then_0
      (if (CallFunction|IsOffCooldown (Variables|Default|GetSpawnCooldown) (Variables|Default|GetCooldowns))
        (CallFunction|SpawnMeteor)))
    (:then_1
      (CallFunction|UpdateCooldowns (Utilities|Time|GetWorldDeltaSeconds) (Variables|Default|GetCooldowns)))))

(fn ConstructionScript)

(fn SpawnMeteor)
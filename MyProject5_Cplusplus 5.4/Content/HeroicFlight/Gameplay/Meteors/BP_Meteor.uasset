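; Meteor projectile actor that either crashes into surfaces or is destroyed in the air by damage.
; Spawns a Niagara comet trail on BeginPlay, moving it with the actor each Tick while spinning the rock and fire dome.
; A sphere hit spawns a shockwave aligned to the impact normal, while depleted health triggers an explosion oriented along projectile velocity.
; Both paths deactivate the trail and destroy the actor.
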(event OnComponentHit(Sphere)
  (params (HitComponent :type Primitive%20Component%20Object%20Reference) (OtherActor :type Actor%20Object%20Reference) (OtherComp :type Primitive%20Component%20Object%20Reference) (NormalImpulse :type Vector :default "0, 0, 0") (Hit :type Hit%20Result%20Structure%20%28by%20ref%29))
  (bind (_bblockinghit _binitialoverlap _time _distance _location _impactpoint _normal _impactnormal) (Collision|BreakHitResult Hit))
  (Niagara|SpawnSystematLocation "/Game/HeroicFlight/VFX/Meteor/NS_FloorShockwave.NS_FloorShockwave" _location (Math|Rotator|MakeRotationfromAxes "0, 0, 0" "0, 0, 0" _impactnormal))
  (CallFunction|OnDestruction))

(event EventBeginPlay
  (Variables|Default|SetHealth (Variables|Default|GetHealthMax))
  (bind _returnvalue (Niagara|SpawnSystematLocation "/Game/HeroicFlight/VFX/Meteor/NS_CometTrail.NS_CometTrail" (Transformation|GetActorLocation) (Transformation|GetActorRotation)))
  (Variables|Default|SetTrail _returnvalue))

(event Collision|EventActorBeginOverlap
  (params (OtherActor :type Actor%20Object%20Reference)))

(event EventTick
  (params (DeltaSeconds :type Float%20%28single-precision%29))
  (Transformation|AddWorldRotation (Variables|Default|GetRockRotatingContainer) (* (Math|Rotator|MakeRotator -1e+02 0.0 0.0) (* DeltaSeconds 5.0)) false false)
  (Transformation|AddRelativeRotation (Variables|Default|GetFireDome) (* (Math|Rotator|MakeRotator -1e+02 0.0 0.0) (* DeltaSeconds 0.5)) false false)
  (Transformation|SetWorldLocation (Variables|Default|GetTrail) (Transformation|GetActorLocation) false true))

(event Game|Damage|EventAnyDamage
  (params (Damage :type Float%20%28single-precision%29) (DamageType :type Damage%20Type%20Object%20Reference) (InstigatedBy :type Controller%20Object%20Reference) (DamageCauser :type Actor%20Object%20Reference))
  (if (> (Variables|Default|GetHealth) 0.0)
    (bind _output_get (Variables|Default|SetHealth (- (Variables|Default|GetHealth) Damage)))
    (if (<= _output_get 0.0)
      (CallFunction|DamageDestruction))))

(fn ConstructionScript)

(fn DamageDestruction
  (Niagara|SpawnSystematLocation "/Game/HeroicFlight/VFX/Meteor/NS_MeteorExplosion.NS_MeteorExplosion" (Transformation|GetActorLocation) (Math|Conversions|RotationFromXVector (Variables|/Script/Engine.MovementComponent|GetVelocity (Variables|Default|GetProjectileMovement))))
  (CallFunction|OnDestruction))

(fn OnDestruction
  (Components|Activation|Deactivate (Variables|Default|GetTrail))
  (Actor|DestroyActor))
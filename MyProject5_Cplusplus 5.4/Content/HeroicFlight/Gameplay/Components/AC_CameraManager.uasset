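; Camera manager component for the flying character that runs a priority-ordered stack of camera behavior objects.
; Flying mode, focused aiming and boost take-off add or remove behaviors; lower priority numbers take precedence.
; Each tick updates every behavior, but only the top one drives control rotation, spring arm, FOV and pitch limits.
; Removals restore the newly active behavior, and helpers expose camera-input timing, cooldowns, easing and interpolation.
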(event Custom|OnBoostTakeOff
  (BehaviorManagement|AddBehavior "/Game/HeroicFlight/Camera/Behaviors/CM_BoostTakeOff.CM_BoostTakeOff_C" true 2)
  (Utilities|FlowControl|Delay 1.0)
  (BehaviorManagement|RemoveBehaviors "/Game/HeroicFlight/Camera/Behaviors/CM_BoostTakeOff.CM_BoostTakeOff_C"))

(event EventBeginPlay
  (CallFunction|Initialize))

(event EventTick
  (params (DeltaSeconds :type Float%20%28single-precision%29))
  (Utilities|FlowControl|Sequence
    (:then_0
      (BehaviorManagement|ManageBehaviors))
    (:then_1
      (BehaviorManagement|RunBehaviors))
    (:then_2
      (Variables|Default|SetLastMovementMode (Variables|/Script/Engine.CharacterMovementComponent|GetMovementMode (Variables|/Script/Engine.Character|GetCharacterMovement (Variables|Default|GetCharacter)))))))

(fn OnUltraBoostStart
  (for _array_element (Variables|Default|GetBehaviors)
    (bind _ascb_flight (Utilities|Casting|CastToCB_Flight _array_element))
    (Variables|/Game/HeroicFlight/Camera/Behaviors/CB_Flight.CB_Flight_C|SetLagSpeedNoAngleMod _ascb_flight 7.0)
    (Variables|/Game/HeroicFlight/Camera/Behaviors/CB_Flight.CB_Flight_C|SetLagSpeedInterp _ascb_flight 0)))

(fn GetTimeSinceLastCameraInput
  (return (- (Utilities|Time|GetTimeSeconds) (Variables|Default|GetLast%20camera%20input%20time))))

(fn ResetLastInputDelay
  (Variables|Default|SetLast%20camera%20input%20time (Utilities|Time|GetTimeSeconds)))

(fn ForceCameraLock
  (Variables|Default|SetLast%20camera%20input%20time (- (Utilities|Time|GetTimeSeconds) 1e+02)))

(fn UpdateCooldownsInterface
  (params (DeltaTime :type Float%20%28double-precision%29) (Cooldown%20Array :type Array%20of%20BP%20Cooldown%20Object%20References))
  (CallFunction|UpdateCooldowns DeltaTime Cooldown%20Array))

(fn IsonCooldownInterface
  (params (Cooldown%20name :type Name) (Active%20Cooldowns :type Array%20of%20BP%20Cooldown%20Object%20References))
  (return (CallFunction|IsonCooldown Cooldown%20name Active%20Cooldowns)))

(fn StartCooldownInterface
  (params (Name :type Name) (Duration :type Float%20%28double-precision%29) (Array%20to%20fill :type Array%20of%20BP%20Cooldown%20Object%20References))
  (bind (_cooldown _was_created) (CallFunction|StartCooldown self Name Duration Array%20to%20fill))
  (return _cooldown _was_created))

(fn GetTimeSeconds
  (return (Utilities|Time|GetTimeSeconds)))

(fn StartEaseInterface
  (params (Target :type Float%20%28double-precision%29) (Start%20value :type Float%20%28double-precision%29) (Current%20Value :type Float%20%28double-precision%29) (Duration :type Float%20%28double-precision%29) (Easing :type EEasingFunc%20Enum :default "Linear") (Blend%20Exp :type Float%20%28double-precision%29) (Steps :type Integer))
  (bind _ease (CallFunction|StartEase self Target Start%20value Current%20Value Duration Easing Blend%20Exp Steps))
  (return _ease))

(fn IsOffCooldownInterface
  (params (Cooldown%20name :type Name) (Active%20Cooldowns :type Array%20of%20BP%20Cooldown%20Object%20References))
  (return (CallFunction|IsOffCooldown Cooldown%20name Active%20Cooldowns)))

(fn AddBehavior
  (params (Class :type Object%20Class%20Reference) (ReplaceExistingOfClass :type Boolean) (Priority :type Integer))
  (bind _behaviors (Variables|Default|GetBehaviors))
  (CallFunction|Initialize)
  (Utilities|FlowControl|Sequence
    (:then_0
      (if ReplaceExistingOfClass
        (BehaviorManagement|RemoveBehaviors Class)
        (elif (BehaviorManagement|HasBehaviorinStack Class)
          (return))))
    (:then_1
      (bind _returnvalue (Game|ConstructObjectfromClass Class))
      (bind _ascb_base (Utilities|Casting|CastToCB_Base _returnvalue))
      (bind _behavior (Default|Init _ascb_base self (Variables|Default|GetCamera) (Variables|Default|GetCharacter) Priority))
      (Default|StartBlendin _behavior)
      (for (_array_element _array_index) _behaviors
        (if (>= (Variables|/Game/HeroicFlight/Camera/Behaviors/CB_Base.CB_Base_C|GetPriority _array_element) Priority)
          (LocalVariables|SetIndexToInsertAt (+ _array_index 1))))
      (Utilities|Array|Insert _behaviors _behavior (LocalVariables|GetIndexToInsertAt)))))

(fn RemoveBehaviors
  (params (Class :type Object%20Class%20Reference))
  (bind _behavior (BehaviorManagement|GetActiveBehavior))
  (LocalVariables|SetActive%20behavior%20at%20start (BehaviorManagement|GetActiveBehavior))
  (for (_array_element _array_index) (Variables|Default|GetBehaviors)
    (if (== Class (Utilities|GetClass _array_element))
      (Utilities|Array|Add (LocalVariables|GetIndexesToRemove) _array_index)
      (if (== _array_element (BehaviorManagement|GetActiveBehavior))
        (LocalVariables|SetBehaviorBlendingOut _array_element))))
  (for _array_element_2 (LocalVariables|GetIndexesToRemove)
    (Utilities|Array|RemoveIndex (Variables|Default|GetBehaviors) _array_element_2))
  (if (!= _behavior (LocalVariables|GetActive%20behavior%20at%20start))
    (Default|Restore _behavior (LocalVariables|GetBehaviorBlendingOut))))

(fn RunBehaviors
  (bind _returnvalue (Game|GetPlayerCameraManager 0))
  (bind _behavior (BehaviorManagement|GetActiveBehavior))
  (bind _cameradata (Default|GetCameraData _behavior))
  (bind (_desiredcontrolrotation _armlength _armlocation _armsocketoffset _lagspeed _fov _pitchmin _pitchmax) (Utilities|Struct|BreakCameraData _cameradata))
  (if (Utilities|Array|IsNotEmpty (Variables|Default|GetBehaviors))
    (for _array_element (Variables|Default|GetBehaviors)
      (Default|Update _array_element (Utilities|Time|GetWorldDeltaSeconds)))
    (Pawn|SetControlRotation (Pawn|GetController (Variables|Default|GetCharacter)) _desiredcontrolrotation)
    (Variables|/Script/Engine.SpringArmComponent|SetTargetArmLength (Variables|Default|GetCameraSpring) _armlength)
    (Transformation|SetRelativeLocation (Variables|Default|GetCameraSpring) _armlocation false true)
    (Variables|/Script/Engine.SpringArmComponent|SetSocketOffset (Variables|Default|GetCameraSpring) _armsocketoffset)
    (Variables|/Script/Engine.SpringArmComponent|SetCameraLagSpeed (Variables|Default|GetCameraSpring) _lagspeed)
    (Camera|SetFieldOfView (Variables|Default|GetCamera) _fov)
    (Variables|/Script/Engine.PlayerCameraManager|SetViewPitchMin _returnvalue _pitchmin)
    (Variables|/Script/Engine.PlayerCameraManager|SetViewPitchMax _returnvalue _pitchmax)))

(fn HasBehaviorinStack
  (params (Class :type Object%20Class%20Reference))
  (for _array_element (Variables|Default|GetBehaviors)
    (if (== Class (Utilities|GetClass _array_element))
      (return true)))
  (return false))

(fn StartInterpolationInterface
  (params (Target :type Float%20%28double-precision%29) (Start%20Value :type Float%20%28double-precision%29) (InterpolationSpeed :type Float%20%28double-precision%29) (EndInterpolationSpeed%20%28Optional%29 :type Float%20%28double-precision%29) (InterpSpeedInterpolationSpeed%20%28Optional%29 :type Float%20%28double-precision%29))
  (bind _interpolation (CallFunction|StartInterpolation self Target Start%20Value InterpolationSpeed EndInterpolationSpeed%20%28Optional%29 InterpSpeedInterpolationSpeed%20%28Optional%29))
  (return _interpolation))

(fn JustChangedtoMovementMode
  (params (Mode :type EMovementMode%20Enum :default "MOVE_None"))
  (return (and (Utilities|Enum|Equal(Enum) (Variables|/Script/Engine.CharacterMovementComponent|GetMovementMode (Variables|/Script/Engine.Character|GetCharacterMovement (Variables|Default|GetCharacter))) Mode) (Utilities|Enum|NotEqual(Enum) (Variables|Default|GetLastMovementMode) Mode))))

(fn JustLeftMovementMode
  (params (Mode :type EMovementMode%20Enum :default "MOVE_None"))
  (return (and (Utilities|Enum|Equal(Enum) (Variables|Default|GetLastMovementMode) Mode) (Utilities|Enum|NotEqual(Enum) (Variables|/Script/Engine.CharacterMovementComponent|GetMovementMode (Variables|/Script/Engine.Character|GetCharacterMovement (Variables|Default|GetCharacter))) Mode))))

(fn GetActiveBehavior
  (bind _behaviors (Variables|Default|GetBehaviors))
  (bind _returnvalue (Utilities|Array|Length _behaviors))
  (if (> _returnvalue 0)
    (return (Utilities|Array|Get(acopy) _behaviors (- _returnvalue 1)))
    (else
      (return 0))))

(fn ManageBehaviors
  (Utilities|FlowControl|Sequence
    (:then_0
      ;[1 1 1] Flight cam
      (if (CallFunction|JustChangedtoMovementMode "MOVE_Flying")
        (BehaviorManagement|AddBehavior "/Game/HeroicFlight/Camera/Behaviors/CB_Flight.CB_Flight_C" false 2)
        (elif (CallFunction|JustLeftMovementMode "MOVE_Flying")
          (BehaviorManagement|RemoveBehaviors "/Game/HeroicFlight/Camera/Behaviors/CB_Flight.CB_Flight_C"))))
    (:then_1
      (if (Variables|/Game/HeroicFlight/Gameplay/Components/AC_Flight.AC_Flight_C|GetIsFocusedAiming (Variables|Default|GetAC_Flight))
        (BehaviorManagement|AddBehavior "/Game/HeroicFlight/Camera/Behaviors/CB_LaserAim.CB_LaserAim_C" false 1)
        (else
          (BehaviorManagement|RemoveBehaviors "/Game/HeroicFlight/Camera/Behaviors/CB_LaserAim.CB_LaserAim_C"))))))

(fn Initialize
  (if (not (Variables|Default|GetInitialized))
    (Variables|Default|SetInitialized true)
    (bind _ascharacter (Utilities|Casting|CastToCharacter (Components|GetOwner)))
    (bind _output_get (Variables|Default|SetCharacter _ascharacter))
    (Variables|Default|SetAC_Flight (Actor|GetComponentbyClass _output_get "/Game/HeroicFlight/Gameplay/Components/AC_Flight.AC_Flight_C"))
    (Variables|Default|SetCameraSpring (Actor|GetComponentbyClass _output_get "/Script/Engine.SpringArmComponent"))
    (Variables|Default|SetCamera (Variables|/Game/HeroicFlight/Gameplay/Components/AC_Flight.AC_Flight_C|GetCamera (Variables|Default|GetAC_Flight)))))
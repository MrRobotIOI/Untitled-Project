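; Player controller component that routes Enhanced Input actions to the possessed character's AC_Flight component for flight, combat, camera and emote control.
; OnPossess caches the character, its AC_Flight and the owning controller, printing an error if that component is missing.
; Movement is camera-relative; while flying above a speed threshold, lateral move input is dropped and strafe input feeds AC_Flight instead.
; Look input also resets the camera manager's last-input delay.
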(event Custom|OnPossess
  (params (Possessed%20character :type Character%20Object%20Reference))
  (bind _output_get (Variables|Default|SetPlayerCharacter Possessed%20character))
  (Utilities|IsValid (Actor|GetComponentbyClass _output_get "/Game/HeroicFlight/Gameplay/Components/AC_Flight.AC_Flight_C")
    (:Is%20Valid
      (Variables|Default|SetAC_Flight (Actor|GetComponentbyClass _output_get "/Game/HeroicFlight/Gameplay/Components/AC_Flight.AC_Flight_C"))
      (bind _asplayer_controller (Utilities|Casting|CastToPlayerController (Components|GetOwner)))
      (Variables|Default|SetController _asplayer_controller))
    (:Is%20Not%20Valid
      (Development|PrintString "AC_FlightControl Error: The possessed pawn is not a character that has an AC_Flight component"))))

(event Input|EnhancedActionEvents|EnhancedInputActionIA_Move
  (params (ActionValue :type Vector%202D%20Structure) (ElapsedSeconds :type Float%20%28double-precision%29) (TriggeredSeconds :type Float%20%28double-precision%29) (InputAction :type Input%20Action%20Object%20Reference :default "/Game/HeroicFlight/Inputs/Actions/IA_Move.IA_Move"))
  (bind _ac_flight (Variables|Default|GetAC_Flight))
  (bind _ac_flight_2 (Variables|Default|GetAC_Flight))
  (bind _camera (Variables|/Game/HeroicFlight/Gameplay/Components/AC_Flight.AC_Flight_C|GetCamera _ac_flight))
  (bind _camera_2 (Variables|/Game/HeroicFlight/Gameplay/Components/AC_Flight.AC_Flight_C|GetCamera _ac_flight_2))
  (if (Utilities|Enum|Equal(Enum) (Variables|/Script/Engine.CharacterMovementComponent|GetMovementMode (Variables|/Script/Engine.Character|GetCharacterMovement (Variables|Default|GetPlayerCharacter))) "MOVE_Flying")
    (Class|PawnMovementComponent|AddInputVector (Variables|/Script/Engine.Character|GetCharacterMovement (Variables|Default|GetPlayerCharacter)) (+ (* (Math|Vector|GetForwardVector _camera_2) (.y ActionValue)) (Math|Vector|SelectVector "0, 0, 0" (* (Math|Vector|GetRightVector _camera_2) (.x ActionValue)) (CallFunction|IsStrafeActive))) false)
    (else
      (Class|PawnMovementComponent|AddInputVector (Variables|/Script/Engine.Character|GetCharacterMovement (Variables|Default|GetPlayerCharacter)) (+ (* (Math|Vector|GetForwardVector _camera) (.y ActionValue)) (* (Math|Vector|GetRightVector _camera) (.x ActionValue))) false))))

(event Input|EnhancedActionEvents|EnhancedInputActionIA_Fly
  (params (ActionValue :type Vector%202D%20Structure) (ElapsedSeconds :type Float%20%28double-precision%29) (TriggeredSeconds :type Float%20%28double-precision%29) (InputAction :type Input%20Action%20Object%20Reference :default "/Game/HeroicFlight/Inputs/Actions/IA_Fly.IA_Fly"))
  (Default|AddVerticalMovement (Variables|Default|GetAC_Flight) (.y ActionValue)))

(event Input|EnhancedActionEvents|EnhancedInputActionIA_Boost
  (params (ActionValue :type Boolean) (ElapsedSeconds :type Float%20%28double-precision%29) (TriggeredSeconds :type Float%20%28double-precision%29) (InputAction :type Input%20Action%20Object%20Reference :default "/Game/HeroicFlight/Inputs/Actions/IA_Boost.IA_Boost"))
  (:Started
    (Default|RequestBoost (Variables|Default|GetAC_Flight))))

(event Input|EnhancedActionEvents|EnhancedInputActionIA_Camera_Look
  (params (ActionValue :type Vector%202D%20Structure) (ElapsedSeconds :type Float%20%28double-precision%29) (TriggeredSeconds :type Float%20%28double-precision%29) (InputAction :type Input%20Action%20Object%20Reference :default "/Game/HeroicFlight/Inputs/Actions/IA_Camera_Look.IA_Camera_Look"))
  (Utilities|FlowControl|Sequence
    (:then_0
      (Class|PlayerController|AddYawInput (Variables|Default|GetController) (.x ActionValue))
      (Class|PlayerController|AddPitchInput (Variables|Default|GetController) (.y ActionValue)))
    (:then_1
      (if (or (!= (.x ActionValue) 0.0) (!= (.y ActionValue) 0.0))
        (Default|ResetLastInputDelay (Variables|/Game/HeroicFlight/Gameplay/Components/AC_Flight.AC_Flight_C|GetAC_CameraManager (Variables|Default|GetAC_Flight)))))))

(event Input|EnhancedActionEvents|EnhancedInputActionIA_Emote
  (params (ActionValue :type Boolean) (ElapsedSeconds :type Float%20%28double-precision%29) (TriggeredSeconds :type Float%20%28double-precision%29) (InputAction :type Input%20Action%20Object%20Reference :default "/Game/HeroicFlight/Inputs/Actions/IA_Emote.IA_Emote"))
  (:Started
    (Default|PlayEmote (Variables|Default|GetAC_Flight))))

(event Input|EnhancedActionEvents|EnhancedInputActionIA_Break
  (params (ActionValue :type Boolean) (ElapsedSeconds :type Float%20%28double-precision%29) (TriggeredSeconds :type Float%20%28double-precision%29) (InputAction :type Input%20Action%20Object%20Reference :default "/Game/HeroicFlight/Inputs/Actions/IA_Break.IA_Break"))
  (bind _playercharacter (Variables|Default|GetPlayerCharacter))
  (bind _ac_flight (Variables|Default|GetAC_Flight))
  (bind _charactermovement (Variables|/Script/Engine.Character|GetCharacterMovement _playercharacter))
  (bind _movementmode (Variables|/Script/Engine.CharacterMovementComponent|GetMovementMode _charactermovement))
  (bind _returnvalue (Utilities|Enum|Equal(Enum) _movementmode "MOVE_Flying"))
  (:Triggered
    (if _returnvalue
      (Default|RequestBrake _ac_flight)))
  (:Completed
    (if _returnvalue
      (Default|StopBrake _ac_flight))))

(event Input|EnhancedActionEvents|EnhancedInputActionIA_FlyStrafe
  (params (ActionValue :type Float%20%28double-precision%29) (ElapsedSeconds :type Float%20%28double-precision%29) (TriggeredSeconds :type Float%20%28double-precision%29) (InputAction :type Input%20Action%20Object%20Reference :default "/Game/HeroicFlight/Inputs/Actions/IA_FlyStrafe.IA_FlyStrafe"))
  (:Triggered
    (if (and (Utilities|Enum|Equal(Enum) (Variables|/Script/Engine.CharacterMovementComponent|GetMovementMode (Variables|/Script/Engine.Character|GetCharacterMovement (Variables|Default|GetPlayerCharacter))) "MOVE_Flying") (CallFunction|IsStrafeActive))
      (Default|AddFlightStrafeInput (Variables|Default|GetAC_Flight) (* (Math|Vector|GetRightVector (Variables|/Game/HeroicFlight/Gameplay/Components/AC_Flight.AC_Flight_C|GetCamera (Variables|Default|GetAC_Flight))) ActionValue) :!label _label)))
  (:Completed
    (goto _label)))

(event Input|EnhancedActionEvents|EnhancedInputActionIA_LockTarget
  (params (ActionValue :type Boolean) (ElapsedSeconds :type Float%20%28double-precision%29) (TriggeredSeconds :type Float%20%28double-precision%29) (InputAction :type Input%20Action%20Object%20Reference :default "/Game/HeroicFlight/Inputs/Actions/IA_LockTarget.IA_LockTarget"))
  (bind _ac_flight (Variables|Default|GetAC_Flight))
  (:Started
    (Variables|/Game/HeroicFlight/Gameplay/Components/AC_Flight.AC_Flight_C|GetLockedTarget _ac_flight
      (:then
        (Default|UnlockTarget _ac_flight))
      (:else
        (Default|LockTarget _ac_flight)))))

(event Input|EnhancedActionEvents|EnhancedInputActionIA_LaserFire
  (params (ActionValue :type Boolean) (ElapsedSeconds :type Float%20%28double-precision%29) (TriggeredSeconds :type Float%20%28double-precision%29) (InputAction :type Input%20Action%20Object%20Reference :default "/Game/HeroicFlight/Inputs/Actions/IA_LaserFire.IA_LaserFire"))
  (bind _ac_flight (Variables|Default|GetAC_Flight))
  (:Triggered
    (Default|FireLasers _ac_flight))
  (:Completed
    (Default|StopLasers _ac_flight)))

(event Input|EnhancedActionEvents|EnhancedInputActionIA_FocusAim
  (params (ActionValue :type Vector%202D%20Structure) (ElapsedSeconds :type Float%20%28double-precision%29) (TriggeredSeconds :type Float%20%28double-precision%29) (InputAction :type Input%20Action%20Object%20Reference :default "/Game/HeroicFlight/Inputs/Actions/IA_FocusAim.IA_FocusAim"))
  (bind _ac_flight (Variables|Default|GetAC_Flight))
  (:Started
    (Variables|/Game/HeroicFlight/Gameplay/Components/AC_Flight.AC_Flight_C|SetIsFocusedAiming _ac_flight true))
  (:Completed
    (Variables|/Game/HeroicFlight/Gameplay/Components/AC_Flight.AC_Flight_C|SetIsFocusedAiming _ac_flight false)))

(fn IsStrafeActive
  (return (> (Default|GetSpeed (Variables|Default|GetAC_Flight)) 1.1e+03)))
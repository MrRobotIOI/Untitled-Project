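; BP_FloatEase is a utility that eases a float from a start value to a target over a duration with a selectable easing function.
; Init stores the settings and, for a mid-range current value, estimates elapsed time by stepping alpha by 0.01 while the eased result gets closer.
; Update evaluates the clamped ease, advances time by DeltaTime and returns the value with a target-reached flag.
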(fn Init
  (params (Target :type Float%20%28double-precision%29) (Start%20value :type Float%20%28double-precision%29) (Current%20Value :type Float%20%28double-precision%29) (Duration :type Float%20%28double-precision%29) (Easing :type EEasingFunc%20Enum :default "Linear") (Blend%20Exp :type Float%20%28double-precision%29) (Steps :type Integer))
  (Utilities|FlowControl|Sequence
    (:then_0
      (Variables|Default|SetStartValue Start%20value)
      (Variables|Default|SetTarget Target)
      (Variables|Default|SetDuration Duration)
      (Variables|Default|SetEasing Easing)
      (Variables|Default|SetBlend%20Exp Blend%20Exp)
      (Variables|Default|SetSteps Steps))
    (:then_1
      (if (== Current%20Value (Variables|Default|GetTarget))
        (Variables|Default|SetTimeSpent (Variables|Default|GetDuration))
        (elif (!= Start%20value Current%20Value)
          (LocalVariables|SetLastResult (Variables|Default|GetStartValue))
          (while (LocalVariables|GetisGettingCloser)
            (bind _output_get (LocalVariables|SetisGettingCloser (< (Math|Float|Absolute(Float) (- Current%20Value (Math|Interpolation|Ease (Variables|Default|GetEasing) (LocalVariables|GetAlpha) (Variables|Default|GetStartValue) (Variables|Default|GetTarget) (Variables|Default|GetBlend%20Exp) (Variables|Default|GetSteps)))) (Math|Float|Absolute(Float) (- Current%20Value (LocalVariables|GetLastResult))))))
            (if _output_get
              (LocalVariables|SetLastResult (Math|Interpolation|Ease (Variables|Default|GetEasing) (LocalVariables|GetAlpha) (Variables|Default|GetStartValue) (Variables|Default|GetTarget) (Variables|Default|GetBlend%20Exp) (Variables|Default|GetSteps)))
              (bind _output_get_2 (LocalVariables|SetAlpha (+ (LocalVariables|GetAlpha) 0.01)))
              (if (== _output_get_2 1.0)
                (LocalVariables|SetisGettingCloser false))))
          (Variables|Default|SetTimeSpent (* (LocalVariables|GetAlpha) (Variables|Default|GetDuration))))))))

(fn Update
  (params (DeltaTime :type Float%20%28double-precision%29))
  (LocalVariables|SetReturnedValue (Math|Interpolation|Ease (Variables|Default|GetEasing) (Math|Float|Clamp(Float) (/ (Variables|Default|GetTimeSpent) (Variables|Default|GetDuration))) (Variables|Default|GetStartValue) (Variables|Default|GetTarget) (Variables|Default|GetBlend%20Exp) (Variables|Default|GetSteps)))
  (Variables|Default|SetTimeSpent (+ (Variables|Default|GetTimeSpent) DeltaTime))
  (return (LocalVariables|GetReturnedValue) (Math|Float|NearlyEqual(Float) (LocalVariables|GetReturnedValue) (Variables|Default|GetTarget) 1e-06)))
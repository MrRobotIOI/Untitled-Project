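; BP_FloatInterpolation is a HeroicFlight helper that moves a float toward a target at a constant rate.
; Init stores the start, target, speed and an optional nested interpolator, and Update continues from the last value through UpdateFrom.
; UpdateFrom accepts any current value, lets the nested interpolator adjust the speed first for chained acceleration, then steps with FInterpToConstant, snaps near the target and reports arrival.
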(fn Updatefrom
  (params (Delta%20time :type Float%20%28double-precision%29) (CurrentValue :type Float%20%28double-precision%29))
  (Utilities|FlowControl|Sequence
    (:then_0
      (Variables|Default|SetLastValue CurrentValue))
    (:then_1
      (Utilities|IsValid (Variables|Default|GetInterpSpeedInterpolation)
        (:Is%20Valid
          (bind _updated_value (CallFunction|Updatefrom (Variables|Default|GetInterpSpeedInterpolation) Delta%20time (Variables|Default|GetInterpolationSpeed)))
          (Variables|Default|SetInterpolationSpeed _updated_value))))
    (:then_2
      (Variables|Default|SetLastValue (Math|Interpolation|FInterptoConstant (Variables|Default|GetLastValue) (Variables|Default|GetTarget) Delta%20time (Variables|Default|GetInterpolationSpeed)))
      (if (Math|Float|NearlyEqual(Float) (Variables|Default|GetLastValue) (Variables|Default|GetTarget) 0.001)
        (Variables|Default|SetLastValue (Variables|Default|GetTarget)))
      (return (Variables|Default|GetLastValue) (Math|Float|NearlyEqual(Float) (Variables|Default|GetLastValue) (Variables|Default|GetTarget) 0.001)))))

(fn Init
  (params (Target :type Float%20%28double-precision%29) (StartValue :type Float%20%28double-precision%29) (InterpolationSpeed :type Float%20%28double-precision%29) (InterpSpeedInterpolation :type BP%20Float%20Interpolation%20Object%20Reference))
  (Variables|Default|SetStartValue StartValue)
  (Variables|Default|SetLastValue StartValue)
  (Variables|Default|SetTarget Target)
  (Variables|Default|SetInterpolationSpeed InterpolationSpeed)
  (Variables|Default|SetInterpSpeedInterpolation InterpSpeedInterpolation))

(fn Update
  (params (DeltaTime :type Float%20%28double-precision%29))
  (bind (_updated_value _targetreached) (CallFunction|Updatefrom DeltaTime (Variables|Default|GetLastValue)))
  (return _updated_value _targetreached))
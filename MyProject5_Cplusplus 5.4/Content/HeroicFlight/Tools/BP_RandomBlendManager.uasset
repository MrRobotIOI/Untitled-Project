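; Random blend manager that supplies smoothly wandering float values, eased between random targets within an amplitude range.
; GetRandomBlendValue returns the blend matching frequency, range and easing (compared only against the first entry's easing), or registers a new one.
; Blends live in parallel arrays keyed by index, with no handles for callers.
; Tick advances every blend, starting toward a new random target each time its period (1/frequency) elapses.
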(event Custom|Tick
  (params (DeltaTime :type Float%20%28double-precision%29))
  (CallFunction|UpdateRandomBlends DeltaTime))

(fn UpdateRBValue
  (params (Index :type Integer) (DeltaTime :type Float%20%28double-precision%29))
  (bind _rb_frequencies (Variables|Default|GetRB_Frequencies))
  (bind _rb_timerunning (Variables|Default|GetRB_TimeRunning))
  (bind _output (Utilities|Array|Get(acopy) _rb_frequencies Index))
  (bind _output_2 (Utilities|Array|Get(acopy) _rb_timerunning Index))
  (bind _returnvalue (/ 1.0 _output))
  (bind _returnvalue_2 (/ _output_2 _returnvalue))
  (if (>= _returnvalue_2 1.0)
    (Utilities|Array|SetArrayElem (Variables|Default|GetRB_TimeRunning) Index 0.0 true)
    (Utilities|Array|SetArrayElem (Variables|Default|GetRB_Starts) Index (Utilities|Array|Get(acopy) (Variables|Default|GetRB_Values) Index) true)
    (Utilities|Array|SetArrayElem (Variables|Default|GetRB_Targets) Index (Math|Random|RandomFloatinRange (Utilities|Array|Get(acopy) (Variables|Default|GetRB_AmplitudeMin) Index) (Utilities|Array|Get(acopy) (Variables|Default|GetRB_AmplitudeMax) Index)) true)
    (else
      (Utilities|Array|SetArrayElem (Variables|Default|GetRB_TimeRunning) Index (+ (Utilities|Array|Get(acopy) (Variables|Default|GetRB_TimeRunning) Index) DeltaTime) true)
      (Utilities|Array|SetArrayElem (Variables|Default|GetRB_Values) Index (Math|Interpolation|Ease (Utilities|Array|Get(acopy) (Variables|Default|GetRB_Easing) Index) (Math|Float|Clamp(Float) _returnvalue_2) (Utilities|Array|Get(acopy) (Variables|Default|GetRB_Starts) Index) (Utilities|Array|Get(acopy) (Variables|Default|GetRB_Targets) Index) 2.0)))))

(fn GetRandomBlendValue
  (params (Frequency :type Float%20%28double-precision%29) (AmplitudeMin :type Float%20%28double-precision%29) (AmplitudeMax :type Float%20%28double-precision%29) (Easing :type EEasingFunc%20Enum :default "Linear"))
  (bind _rb_values (Variables|Default|GetRB_Values))
  (bind _returnvalue (Utilities|Array|Length _rb_values))
  (bind _returnvalue_2 (- _returnvalue 1))
  (for (_array_element _array_index) (Variables|Default|GetRB_Frequencies)
    (if (== _array_element Frequency)
      (if (== (Utilities|Array|Get(acopy) (Variables|Default|GetRB_AmplitudeMin) _array_index) AmplitudeMin)
        (if (== (Utilities|Array|Get(acopy) (Variables|Default|GetRB_AmplitudeMax) _array_index) AmplitudeMax)
          (if (== (Math|Conversions|ToInteger(Byte) (Utilities|Array|Get(acopy) (Variables|Default|GetRB_Easing))) (Math|Conversions|ToInteger(Byte) Easing))
            (return (Utilities|Array|Get(acopy) (Variables|Default|GetRB_Values) _array_index)))))))
  (bind _output_get (LocalVariables|SetStart%20value (Math|Random|RandomFloatinRange AmplitudeMin AmplitudeMax)))
  (Utilities|Array|Add (Variables|Default|GetRB_Values) _output_get)
  (Utilities|Array|Add (Variables|Default|GetRB_Starts) _output_get)
  (Utilities|Array|Add (Variables|Default|GetRB_Frequencies) Frequency)
  (Utilities|Array|Add (Variables|Default|GetRB_Targets) (Math|Random|RandomFloatinRange AmplitudeMin AmplitudeMax))
  (Utilities|Array|Add (Variables|Default|GetRB_TimeRunning) 0.0)
  (Utilities|Array|Add (Variables|Default|GetRB_Easing) Easing)
  (Utilities|Array|Add (Variables|Default|GetRB_AmplitudeMin) AmplitudeMin)
  (Utilities|Array|Add (Variables|Default|GetRB_AmplitudeMax) AmplitudeMax)
  (CallFunction|UpdateRBValue _returnvalue_2 0.0)
  (return (Utilities|Array|Get(acopy) _rb_values _returnvalue_2)))

(fn UpdateRandomBlends
  (params (DeltaTime :type Float%20%28double-precision%29))
  (for (_ _array_index) (Variables|Default|GetRB_Frequencies)
    (CallFunction|UpdateRBValue _array_index DeltaTime)))